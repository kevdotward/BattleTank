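; BP_Mortar is the mortar actor, with a turret, a barrel, an aiming component and a health bar widget.
; On BeginPlay it initialises the AimingComponent with the turret and barrel components.
; It then casts the widget component's user widget to WBP_MortarHealthBar and passes itself as MortarRef.
; The Blueprint is setup glue only, with no aiming, firing or damage logic in its graphs.
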(event `self.ReceiveBeginPlay`
  (`TankAimingComponent.Initialise` (`self.AimingComponent`) (`self.MortarTurret`) (`self.MortarBarrel`))
  (`self.InitialiseHealthBarWidget`))

(fn `InitialiseHealthBarWidget`
  (bind _aswbp_mortar_health_bar (cast `/Game/UI/WBP_MortarHealthBar` (`WidgetComponent.GetUserWidgetObject` (`self.Widget`))))
  (set `/Game/UI/WBP_MortarHealthBar.MortarRef` self _aswbp_mortar_health_bar)
  (return))

(fn `UserConstructionScript`)