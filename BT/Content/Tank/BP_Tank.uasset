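; BP_Tank is a player-controllable tank pawn that wires input to movement, aiming and camera.
; On BeginPlay it hands the track meshes to TankMovement and the turret and barrel to TankAiming, which receive drive, turn and fire input.
; Aim axes rotate an azimuth gimbal and spring arm, scaled by delta time and sensitivity.
; The construction script sets spring arm roll inheritance; per-track throttle inputs are left unused.
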(event `self.ReceiveBeginPlay`
  (`TankMovementComponent.Initialise` (`self.TankMovement`) (`self.LeftTankTrack`) (`self.RightTankTrack`))
  (`TankAimingComponent.Initialise` (`self.TankAiming`) (`self.TankTurret`) (`self.TankBarrel`)))

(event `InputAxis|AimAzimuth`
  (params (AxisValue :type "Float (single-precision)"))
  ;[1 1 1] Camera Control Inputs
  (`SceneComponent.K2_AddLocalRotation` (`self.AzimuthGimbal`) (`KismetMathLibrary.MakeRotator` 0.0 0.0 (* AxisValue (`GameplayStatics.GetWorldDeltaSeconds`) (`self.AimAzimuthSensitivity`))) false false))

(event `InputAxis|LeftThrottle`
  (params (AxisValue :type "Float (single-precision)"))
  ;[1 1 1] Tank Track Controls
  ;;[1 0 0] Unused for now
)

(event `InputAxis|MoveForward`
  (params (AxisValue :type "Float (single-precision)"))
  ;[1 1 1] Tank Track Controls
  (`TankMovementComponent.IntendMoveForward` (`self.TankMovement`) AxisValue))

(event `InputAxis|AimAltitude`
  (params (AxisValue :type "Float (single-precision)"))
  ;[1 1 1] Camera Control Inputs
  (`SceneComponent.K2_AddLocalRotation` (`self.SpringArm`) (`KismetMathLibrary.MakeRotator` 0.0 (* AxisValue (`GameplayStatics.GetWorldDeltaSeconds`) (`self.AimElevationSensitivity`))) false false))

(event `InputAxis|RightThrottle`
  (params (AxisValue :type "Float (single-precision)"))
  ;[1 1 1] Tank Track Controls
  ;;[1 0 0] Unused for now
)

(event `InputAxis|TurnRight`
  (params (AxisValue :type "Float (single-precision)"))
  ;[1 1 1] Tank Track Controls
  (`TankMovementComponent.IntendTurnRight` (`self.TankMovement`) AxisValue))

(event `InputAction|Fire`
  (params (Key :type "Key Structure"))
  ;[1 1 1] Fire Control
  (:`Pressed`
    (`TankAimingComponent.Fire` (`self.TankAiming`))))

(fn `UserConstructionScript`
  (set `SpringArmComponent.bInheritRoll` (`self.CameraRollsOnHills`) (`self.SpringArm`)))